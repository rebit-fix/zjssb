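; BP_ZJshop is a shop actor that opens a BP_shop widget in response to a story event.
; On BeginPlay it creates the widget, keeps it in Shop and sets itself as the widget's Father.
; When the 剧情响应 (plot response) Return event fires, it passes ShopItem to the widget, adds it to the player screen and switches input to UI-only focused on the shop.
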(event `self.ReceiveBeginPlay`
  (bind _returnvalue (`|CreateWidget` "/Game/UI/shop/BP_shop.BP_shop_C"))
  (bind _output_get (set `self.shop` _returnvalue))
  (set `/Game/UI/shop/BP_shop.father` self _output_get))

(event `BP_剧情响应_Return`
  (bind _shop (`self.shop`))
  (set `/Game/UI/shop/BP_shop.Item` (`self.shopItem`) (`self.shop`))
  (`UserWidget.AddToPlayerScreen` _shop 0)
  (`WidgetBlueprintLibrary.SetInputMode_UIOnlyEx` (`GameplayStatics.GetPlayerController` 0) _shop))
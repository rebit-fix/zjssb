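; BP_sister is the sister actor that the player collects by interacting at close range.
; On BeginPlay it caches the player's BP_ThirdPersonCharacter and binds to its ED_F interaction dispatcher.
; An interaction within range tags the player "sister", sets HaveSister, clears CanHit and destroys this actor.
; HitbySword applies a horizontal force to the capsule, pushing it away from the hit location.
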(event `self.ReceiveBeginPlay`
  (bind _asbp_third_person_character (cast `/Game/ThirdPerson/Blueprints/BP_ThirdPersonCharacter` (`GameplayStatics.GetPlayerPawn` 0)))
  (bind _output_get (set `self.As BP Third Person Character` _asbp_third_person_character))
  (add `/Game/ThirdPerson/Blueprints/BP_ThirdPersonCharacter.ED_F` _output_get (delegate `ED_F`)))

(event `ED_F`
  (bind _as_bp_third_person_character (`self.As BP Third Person Character`))
  ;[1 1 1] 交互信息
  (if (< (`KismetMathLibrary.VSize` (- (`self.K2_GetActorLocation`) (`self.K2_GetActorLocation` (`self.As BP Third Person Character`)))) 100.0)
    (`KismetArrayLibrary.Array_Add` (`Actor.Tags` _as_bp_third_person_character) "sister")
    (set `/Game/ThirdPerson/Blueprints/BP_ThirdPersonCharacter.can_hit` false _as_bp_third_person_character)
    (set `/Game/ThirdPerson/Blueprints/BP_ThirdPersonCharacter.have_sister` true _as_bp_third_person_character)
    (`self.K2_DestroyActor`)))

(event `/Game/BP_actor_Instense.hit_by_sword`
  (params (location :type "Vector Structure") (force :type "Float (double-precision)"))
  (bind _returnvalue (- (`self.K2_GetActorLocation`) location))
  (`PrimitiveComponent.AddForce` (`self.Capsule`) (* (/ (`KismetMathLibrary.MakeVector` (.x _returnvalue) (.y _returnvalue)) (`KismetMathLibrary.VSizeXY` _returnvalue)) force) "None" false))

(fn `UserConstructionScript`)